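; Game mode for an idle clicker that sets up the main UI and accrues points passively over time.
; On BeginPlay it sets the screen resolution, adds the UI_Main widget to the viewport, shows the mouse cursor and switches to UI-only input.
; A looping one-second timer fires UpdateScore, which adds PointsPerSecond to the Points total.
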(event `self.ReceiveBeginPlay`
  (bind _returnvalue (`GameplayStatics.GetPlayerController` 0))
  ;[1 0.5183 0.6915] Init UI
  (bind _returnvalue_2 (`GameUserSettings.GetGameUserSettings`))
  (`GameUserSettings.SetScreenResolution` _returnvalue_2 (make `IntPoint` 1920 1080))
  (bind _returnvalue_3 (`|CreateWidget` "/Game/Blueprints/UI_Main.UI_Main_C"))
  (`UserWidget.AddToViewport` _returnvalue_3 0)
  (set `PlayerController.bShowMouseCursor` true _returnvalue)
  (`WidgetBlueprintLibrary.SetInputMode_UIOnlyEx` _returnvalue _returnvalue_3)
  (`KismetSystemLibrary.K2_SetTimerDelegate` (delegate `UpdateScore`) 1.0 true))

(event `UpdateScore`
  (set `self.Points` (+ (`self.Points`) (`self.PointsPerSecond`))))

(fn `UserConstructionScript`)